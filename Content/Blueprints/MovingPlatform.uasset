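; A moving platform Blueprint that shuttles its static mesh back and forth along its relative Y axis from BeginPlay onward.
; MoveRight and MoveLeft events call each other in an endless loop, each using MoveComponentTo over TrackDuration, then a WaitTime delay.
; RightDistance and LeftDistance set the endpoints on either side, with no Tick logic involved.
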(event `self.ReceiveBeginPlay`
  (`self.MoveRight`))

(event `MoveRight`
  (`KismetSystemLibrary.MoveComponentTo` (`self.StaticMesh`) (`KismetMathLibrary.MakeVector` 0.0 (`self.rightDistance`)) (struct) false false (`self.trackDuration`))
  (`KismetSystemLibrary.Delay` (`self.waitTime`))
  (`self.MoveLeft`))

(event `MoveLeft`
  (`KismetSystemLibrary.MoveComponentTo` (`self.StaticMesh`) (`KismetMathLibrary.MakeVector` 0.0 (* (`self.leftDistance`) -1.0)) (struct) false false (`self.trackDuration`))
  (`KismetSystemLibrary.Delay` (`self.waitTime`))
  (`self.MoveRight`))

(fn `UserConstructionScript`)