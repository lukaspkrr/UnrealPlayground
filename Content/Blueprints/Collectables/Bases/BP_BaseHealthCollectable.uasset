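; Base Blueprint for health pickups that restore a character's health when collected.
; It overrides OnPickUp to add HealthToAdd to CurrentHealth, clamped between zero and MaxHealth, then calls the parent implementation.
; CanBePickedUp refuses collection when health equals the maximum; it calls the parent check but ignores its result.
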(event `self.OnPickUp`
  (params (Character :type "/Game/ThirdPerson/Blueprints/BP_ThirdPersonCharacter Object Reference"))
  ;[0.05127 0.05127 0.05127] Add picked up health value to character
  (set `/Game/ThirdPerson/Blueprints/BP_ThirdPersonCharacter.CurrentHealth` (`KismetMathLibrary.FClamp` (+ (`/Game/ThirdPerson/Blueprints/BP_ThirdPersonCharacter.CurrentHealth` Character) (`self.HealthToAdd`)) 0.0 (`/Game/ThirdPerson/Blueprints/BP_ThirdPersonCharacter.MaxHealth` Character)) Character)
  (`parent.OnPickUp` Character))

(fn `CanBePickedUp`
  (params (Character :type "/Game/ThirdPerson/Blueprints/BP_ThirdPersonCharacter Object Reference"))
  (returns (CanBePickedUp :type Boolean))
  ;[0.05127 0.05127 0.05127] Define when health pick up can be collectable
  (`parent.CanBePickedUp` Character)
  (if (== (`/Game/ThirdPerson/Blueprints/BP_ThirdPersonCharacter.MaxHealth` Character) (`/Game/ThirdPerson/Blueprints/BP_ThirdPersonCharacter.CurrentHealth` Character))
    (return false)
    (else
      (return true))))

(fn `UserConstructionScript`
  (`parent.UserConstructionScript`))