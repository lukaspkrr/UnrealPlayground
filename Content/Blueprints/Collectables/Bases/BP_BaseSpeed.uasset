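; Base Blueprint for a speed collectable that grants the collecting character a timed sprint.
; On pickup it calls StartSprint on the character with its SprintTime, then runs the parent pickup logic.
; CanBePickedUp calls the parent check but bases its result only on IsSprint, refusing pickup while the character is already sprinting.
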(event `self.OnPickUp`
  (params (Character :type "/Game/ThirdPerson/Blueprints/BP_ThirdPersonCharacter Object Reference"))
  (`/Game/ThirdPerson/Blueprints/BP_ThirdPersonCharacter.Start Sprint` Character (`self.sprintTime`))
  (`parent.OnPickUp` Character))

(fn `CanBePickedUp`
  (params (Character :type "/Game/ThirdPerson/Blueprints/BP_ThirdPersonCharacter Object Reference"))
  (returns (CanBePickedUp :type Boolean))
  (`parent.CanBePickedUp` Character)
  (if (`/Game/ThirdPerson/Blueprints/BP_ThirdPersonCharacter.isSprint` Character)
    (return false)
    (else
      (return true))))

(fn `UserConstructionScript`
  (`parent.UserConstructionScript`))