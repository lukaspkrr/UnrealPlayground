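; Base collectable actor that the third-person character picks up by overlapping its collision sphere.
; Overlap runs CanBePickedUp, true by default, then OnPickUp plays an optional sound and destroys the actor.
; Optional idle motion uses two chained timelines for a looping Z-axis float and a RotationComponent for spin.
; The construction script creates dynamic materials for the light globe and Niagara stars, which BeginPlay tints or removes based on flags.
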(event `self.ReceiveBeginPlay`
  (`self.SetColors`)
  (`self.StartAnimations`))

(event `self.CollisionSphere.OnComponentBeginOverlap`
  (params (OverlappedComponent :type "PrimitiveComponent Object Reference") (OtherActor :type "Actor Object Reference") (OtherComp :type "PrimitiveComponent Object Reference") (OtherBodyIndex :type Integer) (bFromSweep :type Boolean) (SweepResult :type "HitResult Structure (by ref)"))
  ;[0.05127 0.05127 0.05127] Execute OnPlayerOverlap just if Collectable colides with player
  (bind _asbp_third_person_character (cast `/Game/ThirdPerson/Blueprints/BP_ThirdPersonCharacter` OtherActor))
  (`self.onPlayerOverlap` _asbp_third_person_character))

(event `onPlayerOverlap`
  (params (Character :type "/Game/ThirdPerson/Blueprints/BP_ThirdPersonCharacter Object Reference"))
  ;[0.05127 0.05127 0.05127] Verify if collectable can be picked Up
  (bind _canbepickedup (`self.CanBePickedUp` Character))
  (if _canbepickedup
    (`self.OnPickUp` Character)))

(event `OnPickUp`
  (params (Character :type "/Game/ThirdPerson/Blueprints/BP_ThirdPersonCharacter Object Reference"))
  ;[0.05127 0.05127 0.05127] Actions when collectable is picked up
  (bind _pickupsound (`self.PickUpSound`)
    (:`then`
      (`GameplayStatics.PlaySoundAtLocation` _pickupsound (`SceneComponent.K2_GetComponentLocation` (`self.StaticMesh`)) (struct) 1.0 1.0 0.0 null null null null))
    (:`else`
      _))
  (`self.K2_DestroyActor`))

(event `StartAnimations`
  ;[0.05127 0.05127 0.05127] Start animations depends of conditions
  (`|ExecutionSequence`
    (:`then_0`
      (if (`self.FloatAnimation`)
        (`self.StartFloatAnim`)))
    (:`then_1`
      (if (`self.RotateAnimation`)
        (`self.StartRotateAnim`)))))

(event `StartFloatAnim`
  (bind _staticmesh (`self.StaticMesh`))
  ;[0.05127 0.05127 0.05127] Start Loop Z Axis animation
  (bind (_direction _newtrack_3) (`Timeline|TimelineZAxis` :!label _label)
    (:`Update`
      (`SceneComponent.K2_SetRelativeLocation` _staticmesh _newtrack_3 false false))
    (:`Finished`
      (bind (_direction_2 _zaxisreverse) (`Timeline|TimelineZAxisReverse` :!via `ReverseFromEnd`)
        (:`Update`
          (`SceneComponent.K2_SetRelativeLocation` _staticmesh _zaxisreverse false false))
        (:`Finished`
          (goto _label :!via `PlayFromStart`))))))

(event `StartRotateAnim`
  ;[0.05127 0.05127 0.05127] Start Rotate animation
  (set `RotatingMovementComponent.RotationRate` (`KismetMathLibrary.MakeRotator` 0.0 0.0 (`self.RotateSpeed`)) (`self.RotationComponent`)))

(event `SetColors`
  ;[0.05127 0.05127 0.05127] Set or Destroy lightGlobe and Niagra particle if exists
  (`|ExecutionSequence`
    (:`then_0`
      (if (`self.LightGlobe`)
        (`MaterialInstanceDynamic.SetVectorParameterValue` (`self.LightGlobeMaterialRef`) "Color" (`self.LightColor`))
        (else
          (`ActorComponent.K2_DestroyComponent` (`self.LightGlobeMesh`)))))
    (:`then_1`
      (if (`self.Particles`)
        (`MaterialInstanceDynamic.SetVectorParameterValue` (`self.NiagaraMaterialRef`) "Color" (`self.ParticleColor`))
        (else
          (`ActorComponent.K2_DestroyComponent` (`self.StarParticles`)))))))

(fn `CanBePickedUp`
  (params (Character :type "/Game/ThirdPerson/Blueprints/BP_ThirdPersonCharacter Object Reference"))
  (returns (CanBePickedUp :type Boolean))
  (return true))

(fn `UserConstructionScript`
  (bind _returnvalue (`PrimitiveComponent.CreateDynamicMaterialInstance` (`self.LightGlobeMesh`) 0 "/Game/Effects/Materials/M_LightBall.M_LightBall" "None"))
  (set `self.LightGlobeMaterialRef` _returnvalue)
  (bind _returnvalue_2 (`KismetMaterialLibrary.CreateDynamicMaterialInstance` "/Game/Effects/Materials/M_Star.M_Star"))
  (bind _output_get (set `self.NiagaraMaterialRef` _returnvalue_2))
  (`NiagaraComponent.SetVariableMaterial` (`self.StarParticles`) "DynamicMaterial" _output_get))